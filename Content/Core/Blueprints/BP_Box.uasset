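; BP_Box is a box that the player picks up and releases through an Interact event.
; With a free right hand, it disables Cube physics, ignores pawn collision, then a tick later snaps to the first-person mesh's Inventory_L socket and registers as the right-hand item.
; If that hand is occupied, it restores blocking collision and physics, with no explicit detach or clearing of the player's held-item state.
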(event EventInteract
  (params (PlayerRef :type BP%20First%20Person%20Character%20Object%20Reference))
  (if (Variables|/Game/FirstPerson/Blueprints/BP_FirstPersonCharacter.BP_FirstPersonCharacter_C|GetHasItemInHandR PlayerRef)
    (CallFunction|SetupforDetatch)
    (else
      (CallFunction|SetupforPickup)
      (Utilities|FlowControl|DelayUntilNextTick)
      (Transformation|AttachComponentToComponent (Variables|/Game/FirstPerson/Blueprints/BP_FirstPersonCharacter.BP_FirstPersonCharacter_C|GetFirstPersonMesh PlayerRef) "Inventory_L" "SnapToTarget" "SnapToTarget" "KeepRelative" true)
      (Variables|/Game/FirstPerson/Blueprints/BP_FirstPersonCharacter.BP_FirstPersonCharacter_C|SetHasItemInHandR PlayerRef true)
      (Variables|/Game/FirstPerson/Blueprints/BP_FirstPersonCharacter.BP_FirstPersonCharacter_C|SetItemInHandR PlayerRef self))))

(fn ConstructionScript)

(fn SetupforPickup
  (bind _cube (Variables|Default|GetCube))
  (Utilities|FlowControl|Sequence
    (:then_0
      (Collision|SetCollisionProfileName _cube "IgnoreOnlyPawn" true :!class /Script/Engine.PrimitiveComponent))
    (:then_1
      (Physics|SetSimulatePhysics _cube false))))

(fn SetupforDetatch
  (bind _cube (Variables|Default|GetCube))
  (Utilities|FlowControl|Sequence
    (:then_0
      (Collision|SetCollisionProfileName _cube "BlockAllDynamic" true :!class /Script/Engine.PrimitiveComponent))
    (:then_1
      (Physics|SetSimulatePhysics _cube true))))