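; BP_Door is a door that opens only when every lock requirement in its list of IDs is cleared.
; CheckLock_Event takes an ID and lock state, rewrites matching entries in the list, then re-evaluates whether any remain locked.
; The result calls OpenDoor or CloseDoor, which are placeholders: opening only prints a debug message and closing is empty.
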(event Custom|CheckLock_Event
  (params (ID :type Integer) (Lock :type Boolean))
  (bind (_array_element _array_index) (Utilities|Array|ForEachLoopwithBreak (.idsneeded (Variables|Default|GetLock)))
    (:LoopBody
      (if (== (.IDNeeded (Utilities|Struct|BreakS_Lock _array_element)) ID)
        (Utilities|Array|SetArrayElem (.idsneeded (Variables|Default|GetLock)) _array_index (Utilities|Struct|MakeS_Lock ID Lock))))
    (:Completed
      (bind _open (CallFunction|CheckifDoorShouldbeUnlocked))
      (if _open
        (CallFunction|OpenDoor)
        (else
          (CallFunction|CloseDoor))))))

(fn ConstructionScript)

(fn CheckifDoorShouldbeUnlocked
  (for _array_element (.idsneeded (Variables|Default|GetLock))
    (if (.locked _array_element)
      (return false)))
  (return true))

(fn OpenDoor
  (Development|PrintString "Opening Door"))

(fn CloseDoor)