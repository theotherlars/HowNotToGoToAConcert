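; BP_Interactable_Box is an interactable box that can be picked up and placed down.
; PickUp turns off physics and collision on the Cube, then moves it back to the DefaultSceneRoot's world location and rotation while keeping its scale.
; PlaceDown re-enables physics simulation and query-and-physics collision on the Cube.
; The construction script only calls the parent's.
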(event EventPickUp
  (bind _defaultsceneroot (Variables|Default|GetDefaultSceneRoot))
  (bind _cube (Variables|Default|GetCube))
  (bind _returnvalue (Transformation|GetWorldTransform _defaultsceneroot))
  (Physics|SetSimulatePhysics _cube false)
  (Collision|SetCollisionEnabled _cube "NoCollision")
  (Transformation|SetWorldTransform _cube (Math|Transform|MakeTransform (.location _returnvalue) (.rotation _returnvalue) (Transformation|GetWorldScale (Variables|Default|GetCube))) false false))

(event EventPlaceDown
  (bind _cube (Variables|Default|GetCube))
  (Physics|SetSimulatePhysics _cube true)
  (Collision|SetCollisionEnabled _cube "QueryAndPhysics"))

(fn ConstructionScript
  (|CallParentFunction))