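; BP_KeyHole is an interactable keyhole that lets the player unlock a linked door with a matching key in low glow stick light.
; Tick shows its sphere only when the player's glow stick is absent or its light is not bright.
; Interact checks the overlapping player's right-hand key ID and dim glow stick before calling the door's lock check.
; ShowInteract briefly reveals prompt text, and a custom event smoothly yaws it toward the camera.
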(event Custom|CustomEvent
  (params (DeltaSeconds :type Float%20%28single-precision%29))
  (bind _pickuptext (Variables|Default|GetPickUpText))
  (bind _pickuptext_2 (Variables|Default|GetPickUpText))
  (if (not (Variables|/Script/Engine.SceneComponent|GetbHiddenInGame _pickuptext_2)) ; Only proceed if a player is present
    (Transformation|SetRelativeRotation _pickuptext (Math|Rotator|MakeRotator 0.0 0.0 (.yaw (Math|Interpolation|RInterpTo (Variables|/Script/Engine.SceneComponent|GetRelativeRotation _pickuptext) (Math|Rotator|FindLookatRotation (Transformation|GetWorldLocation _pickuptext_2) (Transformation|GetActorLocation (Game|GetPlayerCameraManager 0))) DeltaSeconds 1e+01))) false false)))

(event EventShowInteract
  (bind _pickuptext (Variables|Default|GetPickUpText))
  (Development|SetHiddeninGame _pickuptext false false)
  (Utilities|FlowControl|Delay 0.1)
  (Development|SetHiddeninGame _pickuptext true false))

(event EventTick
  (params (DeltaSeconds :type Float%20%28single-precision%29))
  (bind _sphere (Variables|Default|GetSphere))
  (bind _currentglowstick (Variables|/Game/FirstPerson/Blueprints/BP_FirstPersonCharacter.BP_FirstPersonCharacter_C|GetCurrentGlowStick (Variables|Default|GetPlayer%20Ref))
    (:then
      (if (> (Variables|/Script/Engine.LightComponentBase|GetIntensity (Variables|/Game/Core/Blueprints/BP_GlowStick.BP_GlowStick_C|GetPointLight _currentglowstick)) 1e+02)
        (Rendering|SetVisibility _sphere false false)
        (else
          (Rendering|SetVisibility _sphere true false :!label _label))))
    (:else
      (goto _label))))

(event EventBeginPlay
  (bind _asbp_first_person_character (Utilities|Casting|CastToBP_FirstPersonCharacter (Pawn|GetControlledPawn (Game|GetPlayerController 0))))
  (Variables|Default|SetPlayer%20Ref _asbp_first_person_character))

(event EventInteract
  (params (PlayerRef :type BP%20First%20Person%20Character%20Object%20Reference))
  (bind _array_element (Utilities|Array|ForEachLoopwithBreak (Collision|GetOverlappingActors (Variables|Default|GetCollision) "/Game/FirstPerson/Blueprints/BP_FirstPersonCharacter.BP_FirstPersonCharacter_C" :!class /Script/Engine.PrimitiveComponent))
    (:LoopBody
      (bind _asbp_first_person_character (Utilities|Casting|CastToBP_FirstPersonCharacter _array_element))
      (bind _iteminhandr (Variables|/Game/FirstPerson/Blueprints/BP_FirstPersonCharacter.BP_FirstPersonCharacter_C|GetItemInHandR _asbp_first_person_character)
        (:then
          (bind _asbp_key (Utilities|Casting|CastToBP_Key _iteminhandr))
          (if (and (== (Utilities|Struct|BreakS_Key (Variables|/Game/Core/Blueprints/BP_Key.BP_Key_C|GetKey _asbp_key)) (.idneeded (Variables|Default|GetLock))) (< (Variables|/Script/Engine.LightComponentBase|GetIntensity (Variables|/Game/Core/Blueprints/BP_GlowStick.BP_GlowStick_C|GetPointLight (Variables|/Game/FirstPerson/Blueprints/BP_FirstPersonCharacter.BP_FirstPersonCharacter_C|GetCurrentGlowStick _asbp_first_person_character))) 5e+01))
            (Default|CheckLockEvent (Variables|Default|GetDoor) (Utilities|Struct|BreakS_Key (Variables|/Game/Core/Blueprints/BP_Key.BP_Key_C|GetKey _asbp_key)) false)))
        (:else)))))

(fn ConstructionScript)